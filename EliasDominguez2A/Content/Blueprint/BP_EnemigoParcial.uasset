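; BP_EnemigoParcial is an enemy actor that moves itself and periodically fires BP_ProyectilEnemigo projectiles.
; Tick applies VelocidadEnemigo as a local offset every frame, without delta-time scaling or sweep.
; A looping timer from BeginPlay calls SpawnProyectil, spawning a projectile at the actor's location with zero VelocidadBala.
; Helper functions set the velocity or scale it by AcelerarEnemigos, though neither is called here.
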(event `self.ReceiveBeginPlay`
  (`KismetSystemLibrary.K2_SetTimerDelegate` (delegate `Loop`) 10.0 true))

(event `Loop`
  (`self.SpawnProyectil` (0.0 0.0 0.0)))

(event `self.ReceiveTick`
  (params (DeltaSeconds :type "Float (single-precision)"))
  (`self.K2_AddActorLocalOffset` (`self.VelocidadEnemigo`)))

(fn `Multiplicador`
  (params (VelocidadEnemigo :type "Vector Structure"))
  (returns (Resultado :type "Vector Structure"))
  (return (* VelocidadEnemigo (`self.AcelerarEnemigos`))))

(fn `SetVelocidadEnemigo`
  (params (Input :type "Vector Structure"))
  (set `self.VelocidadEnemigo` Input))

(fn `SpawnProyectil`
  (params (VelocidadBala :type "Vector Structure"))
  (`|SpawnActorFromClass` "/Game/Blueprint/BP_ProyectilEnemigo.BP_ProyectilEnemigo_C" (`KismetMathLibrary.MakeTransform` (`self.K2_GetActorLocation`)) "Undefined" "MultiplyWithRoot" null VelocidadBala null))

(fn `UserConstructionScript`)